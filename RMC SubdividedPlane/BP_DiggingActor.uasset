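; Diggable ground actor built on a subdivided plane mesh, exposing setup and deformation entry points.
; Setup passes the grid counts and sizes to DefineSetup, and runs from both the construction script and BeginPlay.
; Deform wraps DeformMesh but is not called within this Blueprint; both underlying functions are defined outside this graph.
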(event `self.ReceiveBeginPlay`
  (`self.Setup`))

(fn `Deform`
  (`self.DeformMesh`))

(fn `Setup`
  (`self.DefineSetup` (`self.Nx`) (`self.Ny`) (`self.SizeX`) (`self.SizeY`)))

(fn `UserConstructionScript`
  (`self.Setup`))