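; Runtime Mesh Component actor for a dirt hill plane, sized and subdivided by its Nx, Ny and size variables.
; Construction and BeginPlay both create a DirtHillActor provider, define its setup and initialize the mesh with it; the material slot setup is unwired.
; OrientPlane, not called within this Blueprint, line-traces down from four corners and averages opposite-edge slopes to set roll and pitch.
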(event `self.ReceiveBeginPlay`
  (`self.MakeProvider`))

(fn `MakeProvider`
  (bind _returnvalue (`|GenericCreateObject` "/Script/FishersIsle.DirtHillActor" (`self.RuntimeMeshComponent`)))
  (bind _output_get (set `self.DirtHillProvider` _returnvalue))
  (`|ExecutionSequence`
    (:`then_0`
      (`DirtHillActor.DefineSetup` _output_get (`self.Nx`) (`self.Ny`) (`self.SizeX`) (`self.SizeY`)))
    (:`then_1`
      (`RuntimeMeshComponent.Initialize` (`self.RuntimeMeshComponent`) _output_get))))

(fn `OrientPlane`
  (locals (DistTopLeft :type "Float (double-precision)" :default 0.0) (DistTopRight :type "Float (double-precision)" :default 0.0) (DistBottomRight :type "Float (double-precision)" :default 0.0) (DistBottomLeft :type "Float (double-precision)" :default 0.0))
  (bind _returnvalue (`self.K2_GetActorLocation`))
  (bind _returnvalue_2 (+ (`self.K2_GetActorLocation`) (`KismetMathLibrary.MakeVector` 0.0 (`self.SizeY`))))
  (bind _returnvalue_3 (+ (`self.K2_GetActorLocation`) (`KismetMathLibrary.MakeVector` (`self.SizeX`))))
  (bind _returnvalue_4 (+ (`self.K2_GetActorLocation`) (`KismetMathLibrary.MakeVector` (`self.SizeX`) (`self.SizeY`))))
  (`self.K2_SetActorRotation` (struct))
  (`|ExecutionSequence`
    (:`then_0`
      (bind _outhit (`KismetSystemLibrary.LineTraceSingleForObjects` :`Start` _returnvalue :`End` (+ _returnvalue (0.0 0.0 -500.0)) :`ObjectTypes` (`|MakeArray` "ObjectTypeQuery8" :!type "EObjectTypeQuery Enum") :`DrawDebugType` "ForDuration"))
      (set `local.DistTopLeft` (`.Distance` (`GameplayStatics.BreakHitResult` _outhit))))
    (:`then_1`
      (bind _outhit_2 (`KismetSystemLibrary.LineTraceSingleForObjects` :`Start` _returnvalue_3 :`End` (+ _returnvalue_3 (0.0 0.0 -500.0)) :`ObjectTypes` (`|MakeArray` "ObjectTypeQuery8" :!type "EObjectTypeQuery Enum") :`DrawDebugType` "ForDuration"))
      (set `local.DistTopRight` (`.Distance` (`GameplayStatics.BreakHitResult` _outhit_2))))
    (:`then_2`
      (bind _outhit_3 (`KismetSystemLibrary.LineTraceSingleForObjects` :`Start` _returnvalue_4 :`End` (+ _returnvalue_4 (0.0 0.0 -500.0)) :`ObjectTypes` (`|MakeArray` "ObjectTypeQuery8" :!type "EObjectTypeQuery Enum") :`DrawDebugType` "ForDuration"))
      (set `local.DistBottomRight` (`.Distance` (`GameplayStatics.BreakHitResult` _outhit_3))))
    (:`then_3`
      (bind _outhit_4 (`KismetSystemLibrary.LineTraceSingleForObjects` :`Start` _returnvalue_2 :`End` (+ _returnvalue_2 (0.0 0.0 -500.0)) :`ObjectTypes` (`|MakeArray` "ObjectTypeQuery8" :!type "EObjectTypeQuery Enum") :`DrawDebugType` "ForDuration"))
      (set `local.DistBottomLeft` (`.Distance` (`GameplayStatics.BreakHitResult` _outhit_4))))
    (:`then_4`
      (`self.K2_SetActorRotation` (`KismetMathLibrary.MakeRotator` (* (+ (`KismetMathLibrary.DegAtan` (/ (- (`local.DistBottomLeft`) (`local.DistTopLeft`)) (`self.SizeY`))) (`KismetMathLibrary.DegAtan` (/ (- (`local.DistBottomRight`) (`local.DistTopRight`)) (`self.SizeY`)))) 0.5) (* (+ (`KismetMathLibrary.DegAtan` (/ (- (`local.DistBottomLeft`) (`local.DistBottomRight`)) (`self.SizeX`))) (`KismetMathLibrary.DegAtan` (/ (- (`local.DistTopLeft`) (`local.DistTopRight`)) (`self.SizeX`)))) 0.5))))))

(fn `UserConstructionScript`
  (`self.MakeProvider`))